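; Openable door actor that swings open and closed in response to its OpenDoor component's OnOpen and OnClose events.
; BeginPlay caches the starting rotation, and a timeline yaw curve is combined with it to rotate the whole actor.
; Opening plays the timeline, closing reverses it, and a timeline event track plays the door lock sound at the actor's location.
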(event `self.ReceiveBeginPlay`
  (set `self.Initial Rotation` (`self.K2_GetActorRotation`)))

(event `self.OpenDoor.OnOpen`
  (bind (_direction _open_angle) (`Timeline|Timeline_0` :!label _label)
    (:`Update`
      (`self.K2_SetActorRotation` (`KismetMathLibrary.ComposeRotators` (`self.Initial Rotation`) (`KismetMathLibrary.MakeRotator` 0.0 0.0 _open_angle))))
    (:`Door Open`
      (`GameplayStatics.PlaySoundAtLocation` "/Game/door-lock.door-lock" (`self.K2_GetActorLocation`) (struct) 1.0 1.0 0.0 null null null))))

(event `self.OpenDoor.OnClose`
  (goto _label :!via `Reverse`))

(fn `UserConstructionScript`)